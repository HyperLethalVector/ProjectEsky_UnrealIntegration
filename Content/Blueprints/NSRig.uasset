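; NSRig is a Blueprint that hosts a server-side TextureShare for the duration of its play lifetime.
; BeginPlay creates the share from its ShareName and SyncMode variables, and EndPlay releases it by the same name.
; Each Tick applies the Postprocess variable to that share through the TextureShare API.
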(event `self.ReceiveBeginPlay`
  (`TextureShareBlueprintAPI.CreateTextureShare` (`TextureShareIBlueprintLib.GetAPI`) (`self.Share Name`) (`self.SyncMode`) true))

(event `self.ReceiveEndPlay`
  (params (EndPlayReason :type "EEndPlayReason Enum" :default "Destroyed"))
  (`TextureShareBlueprintAPI.ReleaseTextureShare` (`TextureShareIBlueprintLib.GetAPI`) (`self.Share Name`)))

(event `self.ReceiveTick`
  (params (DeltaSeconds :type "Float (single-precision)"))
  (`TextureShareBlueprintAPI.ApplyTextureSharePostprocess` (`TextureShareIBlueprintLib.GetAPI`) (`self.Share Name`) (`self.Postprocess`)))

(fn `UserConstructionScript`)